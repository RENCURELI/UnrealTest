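; AI controller for AIAgent pawns that runs their behavior tree and tracks the player by perception.
; On possess it caches the agent and starts BTAgentTree.
; Perception updates on TestPlayer set the PlayerDetected blackboard key; on losing sight it stores the player's current location in PlayerPos and flags RecentlySighted.
; Walk and Run events forward movement mode changes to the agent.
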(event OnTargetPerceptionUpdated(AIPerception)
  (params (Actor :type Actor%20Object%20Reference) (Stimulus :type AI%20Stimulus%20Structure))
  (bind _bsuccessfullysensed (Utilities|Struct|BreakAIStimulus Stimulus))
  (bind _returnvalue (AI|GetBlackboard 0))
  (Utilities|Casting|CastToTestPlayer Actor)
  (AI|Components|Blackboard|SetValueasBool _returnvalue (Utilities|Name|MakeLiteralName "PlayerDetected") _bsuccessfullysensed)
  (if (not _bsuccessfullysensed)
    (AI|Components|Blackboard|SetValueasVector _returnvalue (Utilities|Name|MakeLiteralName "PlayerPos") (Transformation|GetActorLocation (Game|GetPlayerCharacter 0)))
    (AI|Components|Blackboard|SetValueasBool _returnvalue (Utilities|Name|MakeLiteralName "RecentlySighted") true)))

(event Custom|Walk
  (Default|Walk (Variables|Default|GetAgent)))

(event Custom|Run
  (Default|Run (Variables|Default|GetAgent)))

(event EventPossess
  (params (PossessedPawn :type Pawn%20Object%20Reference))
  (bind _asaiagent (Utilities|Casting|CastToAIAgent PossessedPawn))
  (Variables|Default|SetAgent _asaiagent)
  (AI|RunBehaviorTree (Variables|Default|GetBT_AgentTree)))

(fn ConstructionScript)