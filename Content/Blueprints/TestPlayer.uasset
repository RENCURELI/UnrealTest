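; TestPlayer is a player Character Blueprint that handles basic movement, camera control and a flashlight.
; Input axes drive forward and strafe movement along the actor's forward and right vectors, and feed controller yaw and pitch for looking.
; Jump copies a JumpTime variable into JumpMaxHoldTime on press for hold-based jumping and stops on release, while the FlashLight action toggles the light component's visibility.
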(event Input|ActionEvents|InputActionJump
  (params (Key :type Key%20Structure :default "None"))
  (:Pressed
    (Variables|Default|SetJumpMaxHoldTime (Variables|Default|GetJumpTime))
    (Character|Jump))
  (:Released
    (Character|StopJumping)))

(event Input|ActionEvents|InputActionFlashLight
  (params (Key :type Key%20Structure :default "None"))
  (:Pressed
    (Rendering|ToggleVisibility (Variables|Default|GetFlashLight) false)))

(event Input|AxisEvents|InputAxisForward_Backwards
  (params (AxisValue :type Float%20%28single-precision%29))
  ;[1 1 1] Basic movements
  (Pawn|Input|AddMovementInput (Transformation|GetActorForwardVector) AxisValue false))

(event Input|AxisEvents|InputAxisStrafe
  (params (AxisValue :type Float%20%28single-precision%29))
  ;[1 1 1] Basic movements
  (Pawn|Input|AddMovementInput (Transformation|GetActorRightVector) AxisValue false))

(event Input|AxisEvents|InputAxisRotate
  (params (AxisValue :type Float%20%28single-precision%29))
  ;[1 1 1] Camera controls
  (Pawn|Input|AddControllerYawInput AxisValue))

(event Input|AxisEvents|InputAxisLookUp_Down
  (params (AxisValue :type Float%20%28single-precision%29))
  ;[1 1 1] Camera controls
  (Pawn|Input|AddControllerPitchInput AxisValue))

(fn ConstructionScript)